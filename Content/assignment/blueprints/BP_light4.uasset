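; BP_light4 is an overlap-triggered switch that toggles the spotlights of Light1 and Light3 together.
; Each actor overlap flips Visible4, which decides whether both lights are shown or hidden, with no filter on the overlapping actor.
; It then casts the Chest reference to BP_lightvariableholder and mirrors the new light state into its True1 and True3 flags.
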(event `self.ReceiveActorBeginOverlap`
  (params (OtherActor :type "Actor Object Reference"))
  (if (`self.visible4`)
    (`SceneComponent.SetVisibility` (`SpotLight.SpotLightComponent` (`self.light1`)) true false)
    (`SceneComponent.SetVisibility` (`SpotLight.SpotLightComponent` (`self.light3`)) true false)
    (set `self.visible4` false)
    (bind _asbp_lightvariableholder (cast `/Game/assignment/blueprints/BP_lightvariableholder` (`self.chest`)))
    (set `/Game/assignment/blueprints/BP_lightvariableholder.true1` true _asbp_lightvariableholder)
    (set `/Game/assignment/blueprints/BP_lightvariableholder.true3` true _asbp_lightvariableholder)
    (else
      (`SceneComponent.SetVisibility` (`SpotLight.SpotLightComponent` (`self.light1`)) false false)
      (`SceneComponent.SetVisibility` (`SpotLight.SpotLightComponent` (`self.light3`)) false false)
      (set `self.visible4` true)
      (bind _asbp_lightvariableholder_2 (cast `/Game/assignment/blueprints/BP_lightvariableholder` (`self.chest`)))
      (set `/Game/assignment/blueprints/BP_lightvariableholder.true1` false _asbp_lightvariableholder_2)
      (set `/Game/assignment/blueprints/BP_lightvariableholder.true3` false _asbp_lightvariableholder_2))))

(fn `UserConstructionScript`)