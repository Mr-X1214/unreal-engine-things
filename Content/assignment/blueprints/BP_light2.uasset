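; BP_light2 is an overlap-triggered switch that toggles a pair of referenced spot lights, Light1 and Light5.
; Each actor overlap flips its Visible2 flag and hides or shows both lights' SpotLightComponents to match.
; It then casts the Chest reference to BP_lightvariableholder and writes the same on/off state into its True1 and True5 flags.
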(event `self.ReceiveActorBeginOverlap`
  (params (OtherActor :type "Actor Object Reference"))
  (if (`self.visible2`)
    (`SceneComponent.SetVisibility` (`SpotLight.SpotLightComponent` (`self.light1`)) false false)
    (`SceneComponent.SetVisibility` (`SpotLight.SpotLightComponent` (`self.light5`)) false false)
    (set `self.visible2` false)
    (bind _asbp_lightvariableholder (cast `/Game/assignment/blueprints/BP_lightvariableholder` (`self.chest`)))
    (set `/Game/assignment/blueprints/BP_lightvariableholder.true1` false _asbp_lightvariableholder)
    (set `/Game/assignment/blueprints/BP_lightvariableholder.true5` false _asbp_lightvariableholder)
    (else
      (`SceneComponent.SetVisibility` (`SpotLight.SpotLightComponent` (`self.light1`)) true false)
      (`SceneComponent.SetVisibility` (`SpotLight.SpotLightComponent` (`self.light5`)) true false)
      (set `self.visible2` true)
      (bind _asbp_lightvariableholder_2 (cast `/Game/assignment/blueprints/BP_lightvariableholder` (`self.chest`)))
      (set `/Game/assignment/blueprints/BP_lightvariableholder.true1` true _asbp_lightvariableholder_2)
      (set `/Game/assignment/blueprints/BP_lightvariableholder.true5` true _asbp_lightvariableholder_2))))

(fn `UserConstructionScript`)