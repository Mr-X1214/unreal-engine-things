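; BP_chest is a chest actor that stays hidden until five flags on a BP_lightvariableholder are all true, apparently as the reward for a light puzzle.
; Every Tick it casts its Lightvariables reference to that holder and checks True1 through True5, showing or hiding itself through SetActorHiddenInGame.
; It polls rather than reacting to events, toggles only visibility, and has no overlap or construction logic.
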(event `self.ReceiveTick`
  (params (DeltaSeconds :type "Float (single-precision)"))
  (bind _defaultsceneroot (`self.DefaultSceneRoot`))
  (bind _asbp_lightvariableholder (cast `/Game/assignment/blueprints/BP_lightvariableholder` (`self.lightvariables`)))
  (if (and (`/Game/assignment/blueprints/BP_lightvariableholder.true1` _asbp_lightvariableholder) (`/Game/assignment/blueprints/BP_lightvariableholder.true2` _asbp_lightvariableholder) (`/Game/assignment/blueprints/BP_lightvariableholder.true3` _asbp_lightvariableholder) (`/Game/assignment/blueprints/BP_lightvariableholder.true4` _asbp_lightvariableholder) (`/Game/assignment/blueprints/BP_lightvariableholder.true5` _asbp_lightvariableholder))
    (`self.SetActorHiddenInGame` (`ActorComponent.GetOwner` _defaultsceneroot) false)
    (else
      (`self.SetActorHiddenInGame` (`ActorComponent.GetOwner` _defaultsceneroot) true))))

(fn `UserConstructionScript`)