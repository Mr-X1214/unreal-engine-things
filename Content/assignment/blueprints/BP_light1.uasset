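; BP_light1 is an overlap trigger that toggles two linked spotlights, apparently as one switch in a light puzzle tied to a chest.
; Each ActorBeginOverlap, from any actor, flips Visible1 and shows or hides Light2 and Light5.
; It then casts the Chest reference to BP_lightvariableholder and mirrors the new on/off state into its True2 and True5 flags.
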(event `self.ReceiveBeginPlay`)

(event `self.ReceiveActorBeginOverlap`
  (params (OtherActor :type "Actor Object Reference"))
  (if (`self.visible1`)
    (`SceneComponent.SetVisibility` (`SpotLight.SpotLightComponent` (`self.light2`)) true false)
    (`SceneComponent.SetVisibility` (`SpotLight.SpotLightComponent` (`self.light5`)) true false)
    (set `self.visible1` false)
    (bind _asbp_lightvariableholder (cast `/Game/assignment/blueprints/BP_lightvariableholder` (`self.chest`)))
    (set `/Game/assignment/blueprints/BP_lightvariableholder.true2` true _asbp_lightvariableholder)
    (set `/Game/assignment/blueprints/BP_lightvariableholder.true5` true _asbp_lightvariableholder)
    (else
      (`SceneComponent.SetVisibility` (`SpotLight.SpotLightComponent` (`self.light2`)) false false)
      (`SceneComponent.SetVisibility` (`SpotLight.SpotLightComponent` (`self.light5`)) false false)
      (set `self.visible1` true)
      (bind _asbp_lightvariableholder_2 (cast `/Game/assignment/blueprints/BP_lightvariableholder` (`self.chest`)))
      (set `/Game/assignment/blueprints/BP_lightvariableholder.true2` false _asbp_lightvariableholder_2)
      (set `/Game/assignment/blueprints/BP_lightvariableholder.true5` false _asbp_lightvariableholder_2))))

(fn `UserConstructionScript`)