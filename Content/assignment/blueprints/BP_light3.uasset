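; BP_light3 is an overlap-triggered light switch, apparently one piece of a multi-switch light puzzle.
; Each actor overlap flips its Visible3 flag and shows or hides the spotlights of Light2 and Light4 to match.
; It then casts the Chest reference to BP_lightvariableholder and writes the same on/off state to its True2 and True4 flags.
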(event `self.ReceiveActorBeginOverlap`
  (params (OtherActor :type "Actor Object Reference"))
  (if (`self.visible3`)
    (`SceneComponent.SetVisibility` (`SpotLight.SpotLightComponent` (`self.light2`)) false false)
    (`SceneComponent.SetVisibility` (`SpotLight.SpotLightComponent` (`self.light4`)) false false)
    (set `self.visible3` false)
    (bind _asbp_lightvariableholder (cast `/Game/assignment/blueprints/BP_lightvariableholder` (`self.chest`)))
    (set `/Game/assignment/blueprints/BP_lightvariableholder.true2` false _asbp_lightvariableholder)
    (set `/Game/assignment/blueprints/BP_lightvariableholder.true4` false _asbp_lightvariableholder)
    (else
      (`SceneComponent.SetVisibility` (`SpotLight.SpotLightComponent` (`self.light2`)) true false)
      (`SceneComponent.SetVisibility` (`SpotLight.SpotLightComponent` (`self.light4`)) true false)
      (set `self.visible3` true)
      (bind _asbp_lightvariableholder_2 (cast `/Game/assignment/blueprints/BP_lightvariableholder` (`self.chest`)))
      (set `/Game/assignment/blueprints/BP_lightvariableholder.true2` true _asbp_lightvariableholder_2)
      (set `/Game/assignment/blueprints/BP_lightvariableholder.true4` true _asbp_lightvariableholder_2))))

(fn `UserConstructionScript`)